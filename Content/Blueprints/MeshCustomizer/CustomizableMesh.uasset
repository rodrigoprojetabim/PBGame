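; CustomizableMesh is an actor with an attached widget that lets its mesh be swapped for another.
; On BeginPlay it passes itself and its MeshFamily to the MeshCustomizerWidget hosted in its Widget component.
; SetCustomizableMesh swaps by replacement: it spawns the given actor class at the current transform, ignoring collisions, then destroys itself, rather than changing a mesh component.
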(event EventBeginPlay
  (|CallParentFunction)
  (bind _asmesh_customizer_widget (Utilities|Casting|CastToMeshCustomizerWidget (UserInterface|GetUserWidgetObject (Variables|Default|GetWidget))))
  (Default|InitializeVariables _asmesh_customizer_widget self (Variables|Default|GetMesh%20Family)))

(fn ConstructionScript
  (|CallParentFunction))

(fn SetCustomizableMesh
  (params (New%20Mesh :type Customizable%20Mesh%20Class%20Reference))
  (Game|SpawnActorfromClass New%20Mesh (Transformation|GetActorTransform) "AlwaysSpawn" 0 0)
  (Actor|DestroyActor))