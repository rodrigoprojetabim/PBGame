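; Interactable radio Blueprint that plays a playlist of media through a media sound component, with play/pause, volume and channel controls.
; Channel changes step through the playlist with wraparound, and BeginPlay either auto-plays or pauses after a short delay.
; Opened media seeks to a calculated time, apparently clock-based to mimic a live broadcast, and replays on ending.
; A media control widget receives a reference to the player.
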(event Custom|Play
  ;[1 1 1] Play
  (if (CallFunction|HasMedia)
    (Media|MediaPlayer|Play (Utilities|GetMediaPlayer) :!class /Script/MediaAssets.MediaPlayer)
    (Media|MediaPlayer|BindEventtoOnMediaOpened (Utilities|GetMediaPlayer) (delegate Custom|Medie%20Opened))
    (else
      (CallFunction|NextMedia))))

(event Custom|Medie%20Opened
  (params (OpenedUrl :type String))
  ;[1 1 1] Play
  (Media|MediaPlayer|Seek (Utilities|GetMediaPlayer) (|Calculateseektime))
  (EventDispatchers|AssignOnEndReached (Utilities|GetMediaPlayer) (delegate Custom|On%20End%20Reached)))

(event Custom|On%20End%20Reached
  ;[1 1 1] Play
  (CallFunction|Play))

(event Custom|NextMedia
  ;[1 1 1] Next / previous
  (EventDispatchers|UnbindallEventsfromOnEndReached (Utilities|GetMediaPlayer))
  (bind _returnvalue (Class|MediaPlaylist|Num (Variables|Default|GetPlaylist)))
  (Variables|Default|SetMedia%20Index (Math|Integer|%(Integer) (+ (Variables|Default|GetMedia%20Index) 1) _returnvalue))
  (bind _returnvalue_2 (Utilities|Array|Get(acopy) (Variables|Default|GetPlaylist) (Variables|Default|GetMedia%20Index)))
  (Variables|Default|SetCurrentMedia _returnvalue_2)
  (Media|MediaPlayer|OpenSource (Utilities|GetMediaPlayer) (Variables|Default|GetCurrentMedia))
  (CallFunction|Play))

(event Custom|PreviousMedia
  ;[1 1 1] Next / previous
  (EventDispatchers|UnbindallEventsfromOnEndReached (Utilities|GetMediaPlayer))
  (bind _returnvalue (Class|MediaPlaylist|Num (Variables|Default|GetPlaylist)))
  (Variables|Default|SetMedia%20Index (select (<= (- (Variables|Default|GetMedia%20Index) 1) -1) (- _returnvalue 1) (- (Variables|Default|GetMedia%20Index) 1)))
  (bind _returnvalue_2 (Utilities|Array|Get(acopy) (Variables|Default|GetPlaylist) (Variables|Default|GetMedia%20Index)))
  (Variables|Default|SetCurrentMedia _returnvalue_2)
  (Media|MediaPlayer|OpenSource (Utilities|GetMediaPlayer) (Variables|Default|GetCurrentMedia))
  (CallFunction|Play))

(event EventBeginPlay
  ;[1 0 0] Begin Play
  (|CallParentFunction)
  (bind _returnvalue (Utilities|Array|Get(acopy) (Variables|Default|GetPlaylist) 0))
  (Variables|Default|SetCurrentMedia _returnvalue)
  (|Updatewidgetvars)
  (Utilities|FlowControl|Delay 2.0)
  (if (Variables|Default|GetAuto%20Play)
    (CallFunction|NextMedia)
    (else
      (CallFunction|Pause))))

(event EventVolumePlus
  (Variables|Default|SetVolumeMult (Math|Float|Clamp(Float) (+ (Variables|Default|GetVolumeMult) 0.05)))
  (Audio|Components|Audio|SetVolumeMultiplier (Variables|Default|GetMediaSound) (Variables|Default|GetVolumeMult) :!class /Script/AudioMixer.SynthComponent))

(event EventVolumeMinus
  (Variables|Default|SetVolumeMult (Math|Float|Clamp(Float) (- (Variables|Default|GetVolumeMult) 0.05)))
  (Audio|Components|Audio|SetVolumeMultiplier (Variables|Default|GetMediaSound) (Variables|Default|GetVolumeMult) :!class /Script/AudioMixer.SynthComponent))

(event EventPlayPause
  (if (CallFunction|HasMedia)
    (if (Class|MediaPlayer|IsPaused (Utilities|GetMediaPlayer))
      (CallFunction|Play)
      (else
        (CallFunction|Pause)))
    (else
      (CallFunction|NextMedia))))

(event EventChannelMinus
  (CallFunction|PreviousMedia))

(event EventChannelPlus
  (CallFunction|NextMedia))

(fn ConstructionScript)

(fn Pause
  (Sequencer|Player|Pause (Class|MediaSoundComponent|GetMediaPlayer (Variables|Default|GetMediaSound))))

(fn HasMedia
  (return (not (Utilities|Text|TextIsEmpty (Class|MediaPlayer|GetMediaName (Class|MediaSoundComponent|GetMediaPlayer (Variables|Default|GetMediaSound)))))))

(fn GetMediaNameFormatted
  (return (Utilities|Text|FormatText "{N} - {X}" (Utilities|Text|ToText(Integer) (+ (Variables|Default|GetMedia%20Index) 1) false false) (Class|MediaPlayer|GetMediaName (Class|MediaSoundComponent|GetMediaPlayer (Variables|Default|GetMediaSound))))))

(fn GetObjectName
  (return "Rádio"))