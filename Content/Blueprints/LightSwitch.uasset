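; Interactable light switch, named "Interruptor", that toggles a set of lights and the glow of their fixture meshes.
; BeginPlay takes the initial on/off state from the visibility of the first light.
; Interact flips that state, sets each light's visibility and, nested inside that loop, creates dynamic material instances on every material slot of the LightMeshes actors' static mesh components to drive the EmissiveOn parameter.
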(event EventBeginPlay
  (bind _lights (Variables|Default|GetLights))
  (bind _output (Utilities|Array|Get(acopy) _lights))
  (Utilities|IsValid _output
    (:Is%20Valid
      (Variables|Default|SetIs%20On (Rendering|IsVisible (Variables|/Script/Engine.Light|GetLightComponent _output))))))

(event EventInteract
  (Variables|Default|SetIs%20On (not (Variables|Default|GetIs%20On)))
  (for _array_element (Variables|Default|GetLights)
    (Rendering|SetVisibility (Variables|/Script/Engine.Light|GetLightComponent _array_element) (Variables|Default|GetIs%20On) false)
    (for _array_element_2 (Variables|Default|GetLightMeshes)
      (for _array_element_3 (Actor|GetComponentsByClass _array_element_2 "/Script/Engine.StaticMeshComponent")
        (for _index (range 0 (- (Rendering|Material|GetNumMaterials _array_element_3) 1))
          (bind _returnvalue (Rendering|Material|CreateDynamicMaterialInstance _array_element_3 _index 0 "None" :!class /Script/Engine.PrimitiveComponent))
          (Rendering|Material|SetScalarParameterValue _returnvalue "EmissiveOn" (Math|Conversions|ToFloat(Boolean) (Variables|Default|GetIs%20On)) :!class /Script/Engine.MaterialInstanceDynamic))))))

(fn ConstructionScript)

(fn GetObjectName
  (return "Interruptor"))