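; MaterialCustomizer is an actor with a widget that lets the material and color of a target mesh slot be changed in game.
; On BeginPlay it passes itself and its MaterialFamily to the widget, and if pitched near vertical it turns upright to face the camera horizontally.
; Color edits use a dynamic material instance, material swaps reapply any stored color, and reset reloads the StaticMeshActor's saved state through the ExplorationGameMode, excluding transform.
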(event EventBeginPlay
  (|CallParentFunction)
  (Utilities|FlowControl|Sequence
    (:then_0
      (bind _asmaterial_customizer_widget (Utilities|Casting|CastToMaterialCustomizerWidget (UserInterface|GetUserWidgetObject (Variables|Default|GetWidget))))
      (Default|InitializeVariables _asmaterial_customizer_widget self (Variables|Default|GetMaterial%20Family)))
    (:then_1
      (if (Math|Float|NearlyEqual(Float) (.pitch (Transformation|GetActorRotation)) 9e+01 5.0)
        (Transformation|SetActorRotation (Math|Rotator|MakeRotfromXZ (Math|Vector|Normalize (- (* (CallFunction|GetCameraWorldLocation) "1.000000,1.000000, 0") (* (Transformation|GetActorLocation) "1.000000,1.000000, 0"))) (Math|Vector|MakeVector 0.0 0.0 1e+01)))))))

(fn ConstructionScript)

(fn ChangeColor
  (params (New%20Color :type Linear%20Color%20Structure))
  (bind _mesh (Variables|Default|GetMesh))
  (bind (_mesh_2 _materialindex _parametername) (Utilities|Struct|BreakMaterialCustomizerMesh _mesh))
  (Variables|Default|SetCurrentColor New%20Color)
  (bind _returnvalue (Rendering|Material|CreateDynamicMaterialInstance _mesh_2 _materialindex 0 "None" :!class /Script/Engine.PrimitiveComponent))
  (Rendering|Material|SetVectorParameterValue _returnvalue _parametername (Variables|Default|GetCurrentColor) :!class /Script/Engine.MaterialInstanceDynamic))

(fn GetObjectName
  (return ""))

(fn SetMaterial
  (params (New%20Materiral :type Material%20Interface%20Object%20Reference))
  (bind _mesh (Variables|Default|GetMesh))
  (bind (_mesh_2 _materialindex) (Utilities|Struct|BreakMaterialCustomizerMesh _mesh))
  (Rendering|Material|SetMaterial _mesh_2 _materialindex New%20Materiral)
  (if (!= (.A (Utilities|Struct|BreakLinearColor (Variables|Default|GetCurrentColor))) -1.0)
    (CallFunction|ChangeColor (Variables|Default|GetCurrentColor))))

(fn ResetMaterial
  (bind _asstatic_mesh_actor (Utilities|Casting|CastToStaticMeshActor (Components|GetOwner (.Mesh (Utilities|Struct|BreakMaterialCustomizerMesh (Variables|Default|GetMesh))))))
  (Default|LoadSMAState (CallFunction|GetExplorationGameMode) _asstatic_mesh_actor false))