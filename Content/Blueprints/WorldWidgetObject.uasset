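; World-space widget actor that pops up when the player approaches and turns to face the camera every tick.
; InteractionBox overlaps play or reverse a timeline that scales the widget between zero and its initial size.
; AlwaysShow disables the box and shows the widget from BeginPlay.
; OnlyShowWidgetIfCustomizationModeIsOn gates overlap transitions on an interface query to the player pawn.
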(event OnComponentBeginOverlap(InteractionBox)
  (params (OverlappedComponent :type Primitive%20Component%20Object%20Reference) (OtherActor :type Actor%20Object%20Reference) (OtherComp :type Primitive%20Component%20Object%20Reference) (OtherBodyIndex :type Integer) (bFromSweep :type Boolean) (SweepResult :type Hit%20Result%20Structure%20%28by%20ref%29))
  ;[1 1 1] Widget scale animation
  (if (Variables|Default|GetOnly%20show%20widget%20if%20Customization%20Mode%20is%20on)
    (bind _return (Class|VisPawnInterface|IsCustomizationModeon(Message) (Game|Player|GetPlayerPawn 0)))
    (if _return
      (bind _newtrack_0 (Timeline|Timeline_0 Play)
        (:Update
          _)
        (:Finished
          _))
      (Transformation|SetRelativeScale3D (Variables|Default|GetWidget) (Math|Vector|Lerp(Vector) "0, 0, 0" (Variables|Default|GetInitial%20Scale) _newtrack_0))
      (Class|WidgetComponent|SetDrawSize (Variables|Default|GetWidget) "(X=1500.000000,Y=1500.000000)"))
    (else
      (Timeline|Timeline_0 Play))))

(event OnComponentEndOverlap(InteractionBox)
  (params (OverlappedComponent :type Primitive%20Component%20Object%20Reference) (OtherActor :type Actor%20Object%20Reference) (OtherComp :type Primitive%20Component%20Object%20Reference) (OtherBodyIndex :type Integer))
  ;[1 1 1] Widget scale animation
  (if (Variables|Default|GetOnly%20show%20widget%20if%20Customization%20Mode%20is%20on)
    (bind _return (Class|VisPawnInterface|IsCustomizationModeon(Message) (Game|Player|GetPlayerPawn 0)))
    (if _return
      (bind _newtrack_0 (Timeline|Timeline_0 Reverse)
        (:Update
          _)
        (:Finished
          _))
      (Transformation|SetRelativeScale3D (Variables|Default|GetWidget) (Math|Vector|Lerp(Vector) "0, 0, 0" (Variables|Default|GetInitial%20Scale) _newtrack_0))
      (Class|WidgetComponent|SetDrawSize (Variables|Default|GetWidget) "(X=1500.000000,Y=1500.000000)"))
    (else
      (Timeline|Timeline_0 Reverse))))

(event Custom|Widget%20Startup
  ;[1 1 1] Widget scale animation
  (Utilities|FlowControl|Delay 0.0)
  (Components|Timeline|SetPlayRate (Variables|Default|GetTimeline_0) (Variables|Default|GetAnimation%20play%20rate))
  (Components|Timeline|SetNewTime (Variables|Default|GetTimeline_0) 0.0)
  (if (or (> (Utilities|Array|Length (Collision|GetOverlappingActors (Variables|Default|GetInteractionBox) "/Script/Engine.Pawn" :!class /Script/Engine.PrimitiveComponent)) 0) (Variables|Default|GetAlways%20Show))
    (bind _newtrack_0 (Timeline|Timeline_0 Play)
      (:Update
        _)
      (:Finished
        _))
    (Transformation|SetRelativeScale3D (Variables|Default|GetWidget) (Math|Vector|Lerp(Vector) "0, 0, 0" (Variables|Default|GetInitial%20Scale) _newtrack_0))
    (Class|WidgetComponent|SetDrawSize (Variables|Default|GetWidget) "(X=1500.000000,Y=1500.000000)")
    (else
      (Timeline|Timeline_0 Reverse))))

(event EventTick
  (params (DeltaSeconds :type Float%20%28single-precision%29))
  ;[1 0.8762 0] Tick
  (|Rotatewidgettocamera))

(event EventBeginPlay
  ;[1 0 0] Begin Play
  (Variables|Default|SetInitial%20Scale (Variables|/Script/Engine.SceneComponent|GetRelativeScale3D (Variables|Default|GetWidget)))
  (Transformation|SetRelativeScale3D (Variables|Default|GetWidget) "0, 0, 0")
  (Rendering|SetVisibility (Variables|Default|GetWidget) true false)
  (CallFunction|WidgetStartup)
  (if (Variables|Default|GetAlways%20Show)
    (Collision|SetCollisionEnabled (Variables|Default|GetInteractionBox) "NoCollision")))

(fn ConstructionScript)

(fn GetObjectName
  (return ""))