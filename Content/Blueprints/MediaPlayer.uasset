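; Interactable in-world radio ("Rádio") that plays a looping playlist of media sources through a MediaSound component, optionally on begin play.
; Interact and channel events switch tracks with wraparound, alongside play/pause and volume controls.
; Opened media seeks via CalculateSeekTime, whose nodes derive a position from wall-clock time modulo duration, like a live broadcast.
; A camera-facing widget scales in and out by timeline on InteractionBox overlap.
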(event OnComponentBeginOverlap(InteractionBox)
  (params (OverlappedComponent :type Primitive%20Component%20Object%20Reference) (OtherActor :type Actor%20Object%20Reference) (OtherComp :type Primitive%20Component%20Object%20Reference) (OtherBodyIndex :type Integer) (bFromSweep :type Boolean) (SweepResult :type Hit%20Result%20Structure%20%28by%20ref%29))
  ;[1 1 1] Widget scale animation
  (bind _newtrack_0 (Timeline|Timeline_0 Play)
    (:Update
      _)
    (:Finished
      _))
  (Transformation|SetRelativeScale3D (Variables|Default|GetWidget) (Math|Vector|Lerp(Vector) "0, 0, 0" (Variables|Default|GetInitial%20Scale) _newtrack_0)))

(event OnComponentEndOverlap(InteractionBox)
  (params (OverlappedComponent :type Primitive%20Component%20Object%20Reference) (OtherActor :type Actor%20Object%20Reference) (OtherComp :type Primitive%20Component%20Object%20Reference) (OtherBodyIndex :type Integer))
  ;[1 1 1] Widget scale animation
  (bind _newtrack_0 (Timeline|Timeline_0 Reverse)
    (:Update
      _)
    (:Finished
      _))
  (Transformation|SetRelativeScale3D (Variables|Default|GetWidget) (Math|Vector|Lerp(Vector) "0, 0, 0" (Variables|Default|GetInitial%20Scale) _newtrack_0)))

(event Custom|Play
  ;[1 1 1] Play
  (if (CallFunction|HasMedia)
    (Media|MediaPlayer|Play (Utilities|GetMediaPlayer) :!class /Script/MediaAssets.MediaPlayer)
    (Media|MediaPlayer|BindEventtoOnMediaOpened (Utilities|GetMediaPlayer) (delegate Custom|Medie%20Opened))
    (else
      (CallFunction|NextMedia))))

(event Custom|Medie%20Opened
  (params (OpenedUrl :type String))
  ;[1 1 1] Play
  (Media|MediaPlayer|Seek (Utilities|GetMediaPlayer) (|Calculateseektime))
  (EventDispatchers|AssignOnEndReached (Utilities|GetMediaPlayer) (delegate Custom|On%20End%20Reached)))

(event Custom|On%20End%20Reached
  ;[1 1 1] Play
  (CallFunction|Play))

(event Custom|NextMedia
  ;[1 1 1] Next / previous
  (EventDispatchers|UnbindallEventsfromOnEndReached (Utilities|GetMediaPlayer))
  (bind _returnvalue (Class|MediaPlaylist|Num (Variables|Default|GetPlaylist)))
  (Variables|Default|SetMedia%20Index (Math|Integer|%(Integer) (+ (Variables|Default|GetMedia%20Index) 1) _returnvalue))
  (bind _returnvalue_2 (Utilities|Array|Get(acopy) (Variables|Default|GetPlaylist) (Variables|Default|GetMedia%20Index)))
  (Variables|Default|SetCurrentMedia _returnvalue_2)
  (Media|MediaPlayer|OpenSource (Utilities|GetMediaPlayer) (Variables|Default|GetCurrentMedia))
  (CallFunction|Play))

(event Custom|PreviousMedia
  ;[1 1 1] Next / previous
  (EventDispatchers|UnbindallEventsfromOnEndReached (Utilities|GetMediaPlayer))
  (bind _returnvalue (Class|MediaPlaylist|Num (Variables|Default|GetPlaylist)))
  (Variables|Default|SetMedia%20Index (select (<= (- (Variables|Default|GetMedia%20Index) 1) -1) (- _returnvalue 1) (- (Variables|Default|GetMedia%20Index) 1)))
  (bind _returnvalue_2 (Utilities|Array|Get(acopy) (Variables|Default|GetPlaylist) (Variables|Default|GetMedia%20Index)))
  (Variables|Default|SetCurrentMedia _returnvalue_2)
  (Media|MediaPlayer|OpenSource (Utilities|GetMediaPlayer) (Variables|Default|GetCurrentMedia))
  (CallFunction|Play))

(event Custom|Widget%20Startup
  ;[1 1 1] Widget scale animation
  (Components|Timeline|SetPlayRate (Variables|Default|GetTimeline_0) 4.0)
  (Components|Timeline|SetNewTime (Variables|Default|GetTimeline_0) 0.0)
  (bind _newtrack_0 (Timeline|Timeline_0 Reverse)
    (:Update
      _)
    (:Finished
      _))
  (Transformation|SetRelativeScale3D (Variables|Default|GetWidget) (Math|Vector|Lerp(Vector) "0, 0, 0" (Variables|Default|GetInitial%20Scale) _newtrack_0)))

(event EventTick
  (params (DeltaSeconds :type Float%20%28single-precision%29))
  ;[1 0.8762 0] Tick
  (|Rotatewidgettocamera))

(event EventBeginPlay
  ;[1 0 0] Begin Play
  (bind _returnvalue (Utilities|Array|Get(acopy) (Variables|Default|GetPlaylist) 0))
  (Variables|Default|SetCurrentMedia _returnvalue)
  (Variables|Default|SetInitial%20Scale (Variables|/Script/Engine.SceneComponent|GetRelativeScale3D (Variables|Default|GetWidget)))
  (CallFunction|WidgetStartup)
  (if (Variables|Default|GetAuto%20Play)
    (CallFunction|NextMedia)))

(event EventInteract
  (CallFunction|NextMedia))

(event EventVolumePlus
  (Variables|Default|SetVolumeMult (Math|Float|Clamp(Float) (+ (Variables|Default|GetVolumeMult) 0.05)))
  (Audio|Components|Audio|SetVolumeMultiplier (Variables|Default|GetMediaSound) (Variables|Default|GetVolumeMult) :!class /Script/AudioMixer.SynthComponent))

(event EventVolumeMinus
  (Variables|Default|SetVolumeMult (Math|Float|Clamp(Float) (- (Variables|Default|GetVolumeMult) 0.05)))
  (Audio|Components|Audio|SetVolumeMultiplier (Variables|Default|GetMediaSound) (Variables|Default|GetVolumeMult) :!class /Script/AudioMixer.SynthComponent))

(event EventPlayPause
  (if (CallFunction|HasMedia)
    (if (Class|MediaPlayer|IsPaused (Utilities|GetMediaPlayer))
      (CallFunction|Play)
      (else
        (CallFunction|Pause)))
    (else
      (CallFunction|NextMedia))))

(event EventChannelMinus
  (CallFunction|PreviousMedia))

(event EventChannelPlus
  (CallFunction|NextMedia))

(fn ConstructionScript)

(fn Pause
  (Sequencer|Player|Pause (Class|MediaSoundComponent|GetMediaPlayer (Variables|Default|GetMediaSound))))

(fn HasMedia
  (return (not (Utilities|Text|TextIsEmpty (Class|MediaPlayer|GetMediaName (Class|MediaSoundComponent|GetMediaPlayer (Variables|Default|GetMediaSound)))))))

(fn GetMediaNameFormatted
  (return (Utilities|Text|FormatText "{N} - {X}" (Utilities|Text|ToText(Integer) (+ (Variables|Default|GetMedia%20Index) 1) false false) (Class|MediaPlayer|GetMediaName (Class|MediaSoundComponent|GetMediaPlayer (Variables|Default|GetMediaSound))))))

(fn GetObjectName
  (return "Rádio"))