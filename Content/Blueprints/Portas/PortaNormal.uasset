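; PortaNormal is a door Blueprint with a Door mesh and a Fixed part, set up as closed or open at construction.
; Its construction script applies MaterialMadeira to both parts, rotates Door to zero or OpenRotation based on StartClosed, and caches its relative location as InitialLocation.
; The event graph has no active logic: Tick is empty and a node that would teleport Door back to InitialLocation is unconnected.
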(event EventTick
  (params (DeltaSeconds :type Float%20%28single-precision%29)))

(fn ConstructionScript
  (Rendering|Material|SetMaterial (Variables|Default|GetDoor) 0 (Variables|Default|GetMaterialMadeira))
  (Transformation|SetRelativeRotation (Variables|Default|GetDoor) (select (Variables|Default|GetStartClosed) "0, 0, 0" (Variables|Default|GetOpenRotation)) false false)
  (Variables|Default|SetInitial%20Location (Variables|/Script/Engine.SceneComponent|GetRelativeLocation (Variables|Default|GetDoor))))