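; Sliding door actor that reports how far open it is; nothing in these graphs moves the door itself.
; The construction script places SlidingDoor at its closed or open position according to StartClosed.
; On Tick, a change in the door's location fires OnMove with a clamped 0–1 value from its world X offset, which ignores actor rotation.
; Nodes for positioning Box1 and Box2 are left disconnected.
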(event EventTick
  (params (DeltaSeconds :type Float%20%28single-precision%29))
  (if (Math|Vector|NotEqual(Vector) (Transformation|GetWorldLocation (Variables|Default|GetSlidingDoor)) (Variables|Default|GetLast%20Location) 0.0001)
    (Variables|Default|SetLast%20Location (Transformation|GetWorldLocation (Variables|Default|GetSlidingDoor)))
    (Default|CallOnMove (Math|Float|Clamp(Float) (- 1.0 (/ (- (.x (Variables|Default|GetLast%20Location)) (.x (Transformation|GetActorLocation))) (- (.x (Variables|Default|GetClosed%20Location)) (.x (Variables|Default|GetOpenLocation)))))))))

(fn ConstructionScript
  (Transformation|SetRelativeLocation (Variables|Default|GetSlidingDoor) (select (Variables|Default|GetStartClosed) (Variables|Default|GetClosed%20Location) (Variables|Default|GetOpenLocation)) false false))