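; Elevator floor button that the player interacts with to send its linked elevator to a given floor.
; SetVariables assigns the floor index and elevator reference, labelling the button "T" for floor zero and one-based numbers for the others.
; Interacting from another floor turns the text white, calls FloorClicked on the elevator and binds to its OnFloorReached event, which turns the text black on arrival at that floor.
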(event Custom|On%20Floor%20Reach
  (params (Floor%20Reached :type Integer))
  (if (== Floor%20Reached (Variables|Default|GetFloor))
    (Rendering|Components|TextRender|SetTextRenderColor (Variables|Default|GetTextRender) (Math|Color|MakeColor 0 0 0 255))))

(event EventInteract
  (bind _elevadorref (Variables|Default|GetElevadorRef))
  (if (!= (Variables|/Game/Blueprints/Elevador/Elevador.Elevador_C|GetCurrent%20Floor (Variables|Default|GetElevadorRef)) (Variables|Default|GetFloor))
    (Rendering|Components|TextRender|SetTextRenderColor (Variables|Default|GetTextRender) (Math|Color|MakeColor 255 255 255 255))
    (Default|FloorClicked _elevadorref (Variables|Default|GetFloor))
    (EventDispatchers|BindEventtoOnFloorReached _elevadorref (delegate Custom|On%20Floor%20Reach))))

(fn ConstructionScript)

(fn SetVariables
  (params (Floor :type Integer) (ElevadorRef :type Elevador%20Object%20Reference))
  (Variables|Default|SetFloor Floor)
  (Variables|Default|SetElevadorRef ElevadorRef)
  (Rendering|Components|TextRender|SetText (Variables|Default|GetTextRender) (select (== (+ (Variables|Default|GetFloor) 1) 1) (Utilities|Text|FormatText "T") (Utilities|Text|ToText(Integer) (+ (Variables|Default|GetFloor) 1)))))

(fn GetObjectName
  (return ""))