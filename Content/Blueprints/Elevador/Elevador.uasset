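; Interactive elevator for a multi-floor Datasmith building, with construction-script buttons and editor placement helpers.
; Button clicks queue floors; with the player inside, a timer counts toward the nearest, then teleports cabin and player there under timeline-driven doors and sounds.
; On arrival it swaps the skybox texture, hides building meshes matched by Datasmith metadata, and toggles ground decoration against one decorated-floor streaming set relocated to the current floor.
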(event Custom|Close%20Door
  ;[1 1 1] On open/close door
  (Variables|Default|SetIs%20Door%20Open false)
  (bind _newtrack_0 (Timeline|OpenClose Reverse)
    (:Update
      (bind _aselevador_skeleton_anim_blueprint (Utilities|Casting|CastToElevador_Skeleton_AnimBlueprint (Components|SkeletalMesh|GetAnimInstance (Variables|Default|GetMesh))))
      (Variables|/Game/ArchVis/Mesh/Predio/Elevador_Skeleton_AnimBlueprint.Elevador_Skeleton_AnimBlueprint_C|SetDoorOpen _aselevador_skeleton_anim_blueprint _newtrack_0))
    (:Finished
      (if (> (Utilities|Array|Length (Variables|Default|GetClicked%20Floors)) 0)
        (if (Variables|Default|GetIs%20Door%20Open)
          (Utilities|FlowControl|Delay (Variables|Default|GetDoor%20Delay))
          (CallFunction|CloseDoor)
          (elif (Collision|IsOverlappingActor (Variables|Default|GetBox) (Game|Player|GetPlayerPawn 0) :!class /Script/Engine.PrimitiveComponent)
            (CallFunction|SetPavementLevelsDecoVisibilityandLocation false "0, 0, 0")
            (CallFunction|SetNextDesiredFloor)
            (Variables|Default|SetIs%20Moving true)
            (bind _returnvalue (Utilities|Time|SetTimerbyEvent (delegate Custom|Move%20One%20Floor) (Variables|Default|GetMove%20Time%20Between%20Floors) true))
            (Variables|Default|SetMove%20One%20Floor%20Timer%20Handle _returnvalue)
            (Audio|PlaySoundatLocation (Variables|Default|GetStart%20Sound) (Transformation|GetActorLocation) "0, 0, 0" 1.0 1.0 0.0 0 0 0)
            (Audio|Components|Audio|FadeIn (Variables|Default|GetLoopingSound) 0.2 1.0 0.0 :!class /Script/Engine.AudioComponent)))))))

(event Custom|Open%20Door
  ;[1 1 1] On open/close door
  (Variables|Default|SetIs%20Door%20Open true)
  (bind _newtrack_0 (Timeline|OpenClose Play)
    (:Update
      (bind _aselevador_skeleton_anim_blueprint (Utilities|Casting|CastToElevador_Skeleton_AnimBlueprint (Components|SkeletalMesh|GetAnimInstance (Variables|Default|GetMesh))))
      (Variables|/Game/ArchVis/Mesh/Predio/Elevador_Skeleton_AnimBlueprint.Elevador_Skeleton_AnimBlueprint_C|SetDoorOpen _aselevador_skeleton_anim_blueprint _newtrack_0))
    (:Finished
      (if (> (Utilities|Array|Length (Variables|Default|GetClicked%20Floors)) 0)
        (if (Variables|Default|GetIs%20Door%20Open)
          (Utilities|FlowControl|Delay (Variables|Default|GetDoor%20Delay))
          (CallFunction|CloseDoor)
          (elif (Collision|IsOverlappingActor (Variables|Default|GetBox) (Game|Player|GetPlayerPawn 0) :!class /Script/Engine.PrimitiveComponent)
            (CallFunction|SetPavementLevelsDecoVisibilityandLocation false "0, 0, 0")
            (CallFunction|SetNextDesiredFloor)
            (Variables|Default|SetIs%20Moving true)
            (bind _returnvalue (Utilities|Time|SetTimerbyEvent (delegate Custom|Move%20One%20Floor) (Variables|Default|GetMove%20Time%20Between%20Floors) true))
            (Variables|Default|SetMove%20One%20Floor%20Timer%20Handle _returnvalue)
            (Audio|PlaySoundatLocation (Variables|Default|GetStart%20Sound) (Transformation|GetActorLocation) "0, 0, 0" 1.0 1.0 0.0 0 0 0)
            (Audio|Components|Audio|FadeIn (Variables|Default|GetLoopingSound) 0.2 1.0 0.0 :!class /Script/Engine.AudioComponent)))))))

(event Custom|Floor%20Clicked
  (params (Floor%20Number :type Integer%20%28by%20ref%29))
  ;[1 1 1] On floor clicked
  (Utilities|Array|AddUnique (Variables|Default|GetClicked%20Floors) Floor%20Number)
  (CallFunction|SetNextDesiredFloor)
  (if (not (Variables|Default|GetIs%20Moving))
    (Utilities|FlowControl|Delay (Variables|Default|GetDoor%20Delay))
    (CallFunction|CloseDoor)))

(event Custom|Move%20One%20Floor
  (bind _current_floor (Variables|Default|GetCurrent%20Floor))
  (bind _returnvalue (+ _current_floor 1))
  ;[1 1 1] Move one floor
  (if (> (Variables|Default|GetNext%20Desired%20Floor) (Variables|Default|GetCurrent%20Floor))
    (Math|Integer|IncrementInt (Variables|Default|GetCurrent%20Floor)
      (:%20%20
        _))
    (else
      (Math|Integer|DecrementInt (Variables|Default|GetCurrent%20Floor)
        (:%20%20
          _))))
  (Rendering|Components|TextRender|SetText (Variables|Default|GetText%20Current%20Floor) (select (== _returnvalue 1) (Utilities|Text|FormatText "T") (Utilities|Text|ToText(Integer) _returnvalue)))
  (if (== (Variables|Default|GetCurrent%20Floor) (Variables|Default|GetNext%20Desired%20Floor))
    (CallFunction|FloorReached (Variables|Default|GetNext%20Desired%20Floor))
    (Utilities|Time|ClearandInvalidateTimerbyHandle (Variables|Default|GetMove%20One%20Floor%20Timer%20Handle))))

(event Custom|Floor%20Reached
  (params (Floor%20reached :type Integer%20%28by%20ref%29))
  ;[1 1 1] On floor reached
  (Utilities|Array|RemoveItem (Variables|Default|GetClicked%20Floors) Floor%20reached)
  (CallFunction|UpdateSkybox)
  (CallFunction|HideBuildingMeshes (+ Floor%20reached 1))
  (CallFunction|MoveDecoratedPavement)
  (Default|CallOnFloorReached Floor%20reached)
  (Variables|Default|SetPlayer%20Position%20Difference (- (Transformation|GetActorLocation (Game|Player|GetPlayerPawn 0)) (Transformation|GetWorldLocation (Variables|Default|GetMesh))))
  (Transformation|SetRelativeLocation (Variables|Default|GetMesh) (CallFunction|CalculatePosition Floor%20reached) false true)
  (Transformation|Teleport (Game|Player|GetPlayerPawn 0) (+ (Transformation|GetWorldLocation (Variables|Default|GetMesh)) (Variables|Default|GetPlayer%20Position%20Difference)) "0, 0, 0")
  (Audio|PlaySoundatLocation (Variables|Default|GetFloor%20Reached%20Sound) (Transformation|GetActorLocation) "0, 0, 0" 1.0 1.0 0.0 0 0 0)
  (Audio|PlaySoundatLocation (Variables|Default|GetEnd%20Sound) (Transformation|GetActorLocation) "0, 0, 0" 1.0 1.0 0.0 0 0 0)
  (Audio|Components|Audio|FadeOut (Variables|Default|GetLoopingSound) 1.0 0.0 :!class /Script/Engine.AudioComponent)
  (Utilities|FlowControl|Delay (Variables|Default|GetDoor%20Delay))
  (CallFunction|OpenDoor)
  (Variables|Default|SetIs%20Moving false))

(event EventBeginPlay
  ;[1 1 1] Begin play
  (|Destroyplacementhelpers)
  (CallFunction|SetGroundLevelsDecoVisibility true)
  (CallFunction|SetPavementLevelsDecoVisibilityandLocation false "0, 0, 0"))

(event EventInteract
  (CallFunction|OpenDoor))

(event Custom|Set%20Ground%20Levels%20Deco%20Visibility2
  (params (bMakeVisibleAfterLoad :type Boolean))
  (for _array_element (Variables|Default|GetGround%20Deco%20levels)
    (Utilities|IsValid (Class|GameplayStatics|GetStreamingLevel _array_element)
      (:Is%20Valid
        (Game|LoadStreamLevel(byName) _array_element bMakeVisibleAfterLoad))
      (:Is%20Not%20Valid
        (Class|ProjetaBimPluginBPLibrary|OpenSystemPopupWarningWindow (Utilities|String|Append "Alerta do BP Elevador: Streaming level \"" (Utilities|String|ToString(Name) _array_element) "\" não encontrado, verifique a variável \"Ground Deco levels\""))
        (Game|QuitGame 0 "Quit")))))

(event Custom|Set%20Pavement%20Levels%20Deco%20Visibility%20and%20Location2
  (params (bMakeVisibleAfterLoad :type Boolean))
  (for _array_element (Variables|Default|GetGround%20Deco%20levels)
    (Utilities|IsValid (Class|GameplayStatics|GetStreamingLevel _array_element)
      (:Is%20Valid
        (Variables|/Script/Engine.LevelStreaming|SetLevelTransform (Class|GameplayStatics|GetStreamingLevel _array_element) (Math|Transform|MakeTransform "0, 0, 0" "0, 0, 0" "1,1,1"))
        (Game|LoadStreamLevel(byName) _array_element bMakeVisibleAfterLoad))
      (:Is%20Not%20Valid
        (Class|ProjetaBimPluginBPLibrary|OpenSystemPopupWarningWindow (Utilities|String|Append "Alerta do BP Elevador: Streaming level \"" (Utilities|String|ToString(Name) _array_element) "\" não encontrado, verifique a variável \"Decorated pavement levels\""))
        (Game|QuitGame 0 "Quit")))))

(fn ConstructionScript
  (LocalVariables|SetCurrent%20Offset (- (Variables|Buttonspositioning|GetFirst%20Button%20Location) (Math|Vector|MakeVector (Variables|Buttonspositioning|GetOffset%20X) 0.0 0.0)))
  (Audio|Components|Audio|SetSound (Variables|Default|GetLoopingSound) (Variables|Default|GetLoop%20Sound))
  (while (< (LocalVariables|GetCurrFloor) (Variables|Default|GetNumFloors))
    (if (LocalVariables|GetSpawn%20Right)
      (LocalVariables|SetCurrent%20Offset (Math|Vector|MakeVector (- (.x (LocalVariables|GetCurrent%20Offset)) (Variables|Buttonspositioning|GetOffset%20X)) (.y (LocalVariables|GetCurrent%20Offset)) (.z (LocalVariables|GetCurrent%20Offset))))
      (else
        (LocalVariables|SetCurrent%20Offset (Math|Vector|MakeVector (+ (.x (LocalVariables|GetCurrent%20Offset)) (Variables|Buttonspositioning|GetOffset%20X)) (.y (LocalVariables|GetCurrent%20Offset)) (.z (LocalVariables|GetCurrent%20Offset))))))
    (LocalVariables|SetSpawn%20Right (not (LocalVariables|GetSpawn%20Right)))
    (bind _returnvalue (AddComponent|AddChildActorComponent true (Math|Transform|MakeTransform (Math|Vector|MakeVector (.x (LocalVariables|GetCurrent%20Offset)) (.y (LocalVariables|GetCurrent%20Offset)) (+ (.z (LocalVariables|GetCurrent%20Offset)) (* (/ (LocalVariables|GetCurrFloor) 2) (Variables|Buttonspositioning|GetOffset%20Z)))) "0, 0, 0" "1,1,1")))
    (Transformation|AttachComponentToComponent _returnvalue (Variables|Default|GetMesh) "None" "KeepRelative" "KeepRelative" "KeepRelative" true)
    (bind _aselevador_botao (Utilities|Casting|CastToElevadorBotao (Variables|/Script/Engine.ChildActorComponent|GetChildActor _returnvalue)))
    (Default|SetVariables _aselevador_botao (LocalVariables|GetCurrFloor) self)
    (Math|Integer|IncrementInt (LocalVariables|GetCurrFloor)))
  ;[1 1 1] placement helpers
  (bind _returnvalue_2 (AddComponent|AddSkeletalMeshComponent true (Math|Transform|MakeTransform (CallFunction|CalculatePosition 1))))
  (Transformation|AttachComponentToComponent _returnvalue_2 (Variables|Default|GetHelpers) "None" "KeepRelative" "KeepRelative" "KeepRelative" true)
  (for _index (range 2 (Variables|Default|GetNumFloors))
    (bind _returnvalue_3 (AddComponent|AddSkeletalMeshComponent true (Math|Transform|MakeTransform (CallFunction|CalculatePosition _index))))
    (Transformation|AttachComponentToComponent _returnvalue_3 (Variables|Default|GetHelpers) "None" "KeepRelative" "KeepRelative" "KeepRelative" true)))

(fn SetNextDesiredFloor
  (LocalVariables|SetLesser%20Difference 99999)
  (for _array_element (Variables|Default|GetClicked%20Floors)
    (if (< (Math|Integer|Absolute(Integer) (- _array_element (Variables|Default|GetCurrent%20Floor))) (LocalVariables|GetLesser%20Difference))
      (Variables|Default|SetNext%20Desired%20Floor _array_element)
      (LocalVariables|SetLesser%20Difference (Math|Integer|Absolute(Integer) (- _array_element (Variables|Default|GetCurrent%20Floor)))))))

(fn CalculatePosition
  (params (Floor%20Number :type Integer))
  (return (select (== Floor%20Number 0) "0, 0, 0" (+ (Variables|FloorOffsets|GetFirst%20Floor%20Offset) (* (Variables|FloorOffsets|GetSubsequent%20Floor%20Offsets) (- Floor%20Number 1))))))

(fn HideBuildingMeshes
  (params (Floor%20to%20hide :type Integer))
  (LocalVariables|SetSearch%20text (Utilities|String|Append (Utilities|String|ToString(Integer) Floor%20to%20hide) (Variables|Default|GetDatasmith%20pavement%20field%20name)))
  (bind _outactors (Actor|GetAllActorsOfClass "/Script/Engine.StaticMeshActor"))
  (for _array_element _outactors
    (bind _output_get (LocalVariables|SetCurrent%20SM _array_element))
    (bind _returnvalue (Class|DatasmithContentBlueprintLibrary|GetDatasmithUserData _output_get))
    (bind _output_get_2 (LocalVariables|SetDatasmith%20user%20data _returnvalue))
    (Utilities|IsValid _output_get_2
      (:Is%20Valid
        (LocalVariables|SetShould%20process false)
        (bind _array_element_2 (Utilities|Array|ForEachLoopwithBreak (Variables|Default|GetLevel%20Names%20to%20hide%20pavement) :!label _label)
          (:LoopBody
            (if (!= (Utilities|String|FindSubstring (Class|ProjetaBimPluginBPLibrary|GetActorsStreamingLevelName (LocalVariables|GetCurrent%20SM)) _array_element_2) -1)
              (LocalVariables|SetShould%20process true)
              (goto _label Break)))
          (:Completed
            (if (LocalVariables|GetShould%20process)
              (for _array_element_3 (Variables|Default|GetDatasmith%20pavement%20tags)
                (if (.ReturnValue (Utilities|Map|Find (Variables|/Script/DatasmithContent.DatasmithAssetUserData|GetMetaData (LocalVariables|GetDatasmith%20user%20data)) _array_element_3))
                  (if (!= (Utilities|String|FindSubstring (.Value (Utilities|Map|Find (Variables|/Script/DatasmithContent.DatasmithAssetUserData|GetMetaData (LocalVariables|GetDatasmith%20user%20data)) _array_element_3)) (LocalVariables|GetSearch%20text)) -1)
                    (Rendering|SetActorHiddenInGame (LocalVariables|GetCurrent%20SM) true)
                    (else
                      (Rendering|SetActorHiddenInGame (LocalVariables|GetCurrent%20SM) false))))))))))))

(fn MoveDecoratedPavement
  (if (== (Variables|Default|GetCurrent%20Floor) 0)
    (CallFunction|SetGroundLevelsDecoVisibility true)
    (CallFunction|SetPavementLevelsDecoVisibilityandLocation false "0, 0, 0")
    (else
      (CallFunction|SetGroundLevelsDecoVisibility false)
      (CallFunction|SetPavementLevelsDecoVisibilityandLocation true (+ (- "0, 0, 0" (CallFunction|CalculatePosition (Variables|Default|GetDecorated%20pavement%20initial%20floor))) (CallFunction|CalculatePosition (Variables|Default|GetCurrent%20Floor)))))))

(fn SetGroundLevelsDecoVisibility
  (params (bShouldBeVisible :type Boolean))
  (for _array_element (Variables|Default|GetGround%20Deco%20levels)
    (Utilities|IsValid (Class|GameplayStatics|GetStreamingLevel _array_element)
      (:Is%20Valid
        (Variables|/Script/Engine.LevelStreaming|SetbShouldBeLoaded (Class|GameplayStatics|GetStreamingLevel _array_element) bShouldBeVisible)
        (Variables|/Script/Engine.LevelStreaming|SetbShouldBeVisible (Class|GameplayStatics|GetStreamingLevel _array_element) bShouldBeVisible)
        (Variables|/Script/Engine.LevelStreaming|SetbShouldBlockOnLoad (Class|GameplayStatics|GetStreamingLevel _array_element) false)
        (Variables|/Script/Engine.LevelStreaming|SetbShouldBlockOnUnload (Class|GameplayStatics|GetStreamingLevel _array_element) false))
      (:Is%20Not%20Valid
        (Class|ProjetaBimPluginBPLibrary|OpenSystemPopupWarningWindow (Utilities|String|Append "Alerta do BP Elevador: Streaming level \"" (Utilities|String|ToString(Name) _array_element) "\" não encontrado, verifique a variável \"Ground Deco levels\""))
        (Game|QuitGame 0 "Quit")))))

(fn SetPavementLevelsDecoVisibilityandLocation
  (params (bShouldBeVisible :type Boolean) (Level%20Transform%20Location :type Vector))
  (for _array_element (Variables|Default|GetDecorated%20pavement%20levels)
    (Utilities|IsValid (Class|GameplayStatics|GetStreamingLevel _array_element)
      (:Is%20Valid
        (Variables|/Script/Engine.LevelStreaming|SetbShouldBeLoaded (Class|GameplayStatics|GetStreamingLevel _array_element) bShouldBeVisible)
        (Variables|/Script/Engine.LevelStreaming|SetLevelTransform (Class|GameplayStatics|GetStreamingLevel _array_element) (Math|Transform|MakeTransform Level%20Transform%20Location "0, 0, 0" "1,1,1"))
        (Variables|/Script/Engine.LevelStreaming|SetbShouldBeVisible (Class|GameplayStatics|GetStreamingLevel _array_element) bShouldBeVisible)
        (Variables|/Script/Engine.LevelStreaming|SetbShouldBlockOnLoad (Class|GameplayStatics|GetStreamingLevel _array_element) false)
        (Variables|/Script/Engine.LevelStreaming|SetbShouldBlockOnUnload (Class|GameplayStatics|GetStreamingLevel _array_element) false))
      (:Is%20Not%20Valid
        (Class|ProjetaBimPluginBPLibrary|OpenSystemPopupWarningWindow (Utilities|String|Append "Alerta do BP Elevador: Streaming level \"" (Utilities|String|ToString(Name) _array_element) "\" não encontrado, verifique a variável \"Decorated pavement levels\""))
        (Game|QuitGame 0 "Quit")))))

(fn UpdateSkybox
  (bind _current_floor (Variables|Default|GetCurrent%20Floor))
  (for _array_element (Variables|Default|GetSkybox%20Textures)
    (if (and (>= _current_floor (.MinFloor (Utilities|Struct|BreakSkyboxOptions _array_element))) (<= _current_floor (.MaxFloor (Utilities|Struct|BreakSkyboxOptions _array_element))))
      (bind _outactors (Actor|GetAllActorswithTag "Skybox"))
      (if (== (Utilities|Array|Length _outactors) 0)
        (Class|ProjetaBimPluginBPLibrary|OpenSystemPopupWarningWindow "Alerta: adicione a Actor Tag \"Skybox\" à skybox do cenário")
        (else
          (bind _asstatic_mesh_component (Utilities|Casting|CastToStaticMeshComponent (Variables|/Script/Engine.Actor|GetRootComponent (Utilities|Array|Get(acopy) _outactors))))
          (bind _returnvalue (Rendering|Material|CreateDynamicMaterialInstance _asstatic_mesh_component 0 0 "None" :!class /Script/Engine.PrimitiveComponent))
          (Rendering|Material|SetTextureParameterValue _returnvalue "Texture" (.SkyboxTexture (Utilities|Struct|BreakSkyboxOptions _array_element))))))))

(fn GetObjectName
  (return ""))